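; levelHUD is a two-player HUD that draws each player's health bar and score on screen every frame.
; DrawHUD casts player characters 0 and 1 to MyCharacter and reads their Health and Score.
; It draws a fill bar whose width scales with Health, layers an HP frame texture over it, then prints labeled scores above.
; Positions and sizes are fractions of screen size, though fill width derives from screen height.
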(event EventDrawHUD
  (params (SizeX :type Integer) (SizeY :type Integer))
  (bind _returnvalue (* SizeY 0.025))
  (bind _returnvalue_2 (* SizeY 0.1505))
  (bind _returnvalue_3 (Math|Conversions|ToFloat(Integer) SizeY))
  (bind _returnvalue_4 (Math|Conversions|ToFloat(Integer) SizeX))
  (bind _returnvalue_5 (|y*0.1 SizeY))
  (bind _returnvalue_6 (|x*0.4 SizeX))
  (bind _returnvalue_7 (|y*0.1 SizeY))
  (Utilities|FlowControl|Sequence
    (:then_0
      (bind _asmycharacter_c (Utilities|Casting|CastToMyCharacter (Game|GetPlayerCharacter 0))))
    (:then_1
      (bind _asmycharacter_c_2 (Utilities|Casting|CastToMyCharacter (Game|GetPlayerCharacter 1))))
    (:then_2
      (Canvas|DrawTexture "/Game/Texture/Life_bar_scale.Life_bar_scale" (* SizeX 0.07) _returnvalue_2 (* (* (Variables|/Game/Blueprints/MyCharacter.MyCharacter_C|GetHealth _asmycharacter_c) 0.006) (Math|Conversions|ToFloat(Integer) SizeY)) _returnvalue 0.0 0.0 1.0 1.0 "(R=1.000000,G=1.000000,B=1.000000,A=1.000000)")
      (Canvas|DrawTexture "/Game/Texture/Life_bar_scale.Life_bar_scale" (* SizeX 0.595) _returnvalue_2 (* (* (Variables|/Game/Blueprints/MyCharacter.MyCharacter_C|GetHealth _asmycharacter_c_2) 0.006) (Math|Conversions|ToFloat(Integer) SizeY)) _returnvalue 0.0 0.0 1.0 1.0 "(R=1.000000,G=1.000000,B=1.000000,A=1.000000)")
      (Canvas|DrawTexture "/Game/Texture/HP_Bar_png_flipped.HP_Bar_png_flipped" (|x*0.05 SizeX) _returnvalue_5 _returnvalue_6 _returnvalue_7 0.0 0.0 1.0 1.0 "(R=1.000000,G=1.000000,B=1.000000,A=1.000000)")
      (Canvas|DrawTexture "/Game/Texture/HP_Bar.HP_Bar" (|x*0.55 SizeX) _returnvalue_5 _returnvalue_6 _returnvalue_7 0.0 0.0 1.0 1.0 "(R=1.000000,G=1.000000,B=1.000000,A=1.000000)"))
    (:then_3
      (bind _asmycharacter_c_3 (Utilities|Casting|CastToMyCharacter (Game|GetPlayerCharacter 0)))
      (HUD|DrawText (Utilities|String|Append (Utilities|String|MakeLiteralString "Player 1: ") (Utilities|String|MakeLiteralString (Utilities|String|ToString(Integer) (Variables|/Game/Blueprints/MyCharacter.MyCharacter_C|GetScore _asmycharacter_c_3)))) "(R=0.000000,G=0.361830,B=1.000000,A=1.000000)" (* _returnvalue_4 0.1) (* _returnvalue_3 0.05) "/Game/Blueprints/Player1_Font.Player1_Font" 1.0 true))
    (:then_4
      (bind _asmycharacter_c_4 (Utilities|Casting|CastToMyCharacter (Game|GetPlayerCharacter 1)))
      (HUD|DrawText (Utilities|String|Append (Utilities|String|MakeLiteralString "Player 2: ") (Utilities|String|MakeLiteralString (Utilities|String|ToString(Integer) (Variables|/Game/Blueprints/MyCharacter.MyCharacter_C|GetScore _asmycharacter_c_4)))) "(R=0.000000,G=0.361830,B=1.000000,A=1.000000)" (* _returnvalue_4 0.8) (* _returnvalue_3 0.05) "/Game/Blueprints/Player1_Font.Player1_Font" 1.0 true))))

(fn ConstructionScript)