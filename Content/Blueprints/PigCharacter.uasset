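; Pig character that stays on a fixed X plane and returns to its placed start location when it falls or respawns.
; The construction script records that location, and Tick snaps X back whenever it drifts beyond a small tolerance.
; Dropping below a Z threshold also restores collision, detaches the pig and clears its held state.
; An explosion effect plays at the start location on BeginPlay and each reset.
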(event EventTick
  (params (DeltaSeconds :type Float%20%28single-precision%29))
  (bind _returnvalue (Transformation|GetActorLocation))
  (bind _lockedx (Variables|Default|GetLockedX))
  (bind _startlocation (Variables|Default|GetStartLocation))
  (bind _startlocation_2 (Variables|Default|GetStartLocation))
  (bind (_x _y _z) (Math|Vector|BreakVector _returnvalue))
  ;[1 1 1] No X movement
  (Utilities|FlowControl|Sequence
    (:then_0
      (if (> _x (+ _lockedx 5.0))
        (Transformation|SetActorLocation (Math|Vector|MakeVector _lockedx _y _z) false :!label _label)))
    (:then_1
      (if (< _x (- _lockedx 5.0))
        (goto _label)))
    (:then_2
      ;[1 1 1] Fell off screen
      (if (< _z 9e+01)
        (Collision|SetCollisionEnabled (Variables|Collision|GetCapsuleComponent) "QueryAndPhysics")
        (Class|Actor|DetachRootComponentfromParent true)
        (Variables|Default|SetisHeld false)
        (Transformation|SetActorLocation _startlocation false)
        (Effects|SpawnEmitteratLocation 0 "/Game/StarterContent/Particles/P_Explosion.P_Explosion" _startlocation)))
    (:then_3
      ;[1 1 1] Respawn
      (if (Variables|Default|GetisRespawn)
        (Transformation|SetActorLocation _startlocation_2 false)
        (Effects|SpawnEmitteratLocation 0 "/Game/StarterContent/Particles/P_Explosion.P_Explosion" _startlocation_2)
        (Variables|Default|SetisRespawn false)))))

(event EventBeginPlay
  ;[1 1 1] Start
  (Effects|SpawnEmitteratLocation 0 "/Game/StarterContent/Particles/P_Explosion.P_Explosion" (Variables|Default|GetStartLocation)))

(fn ConstructionScript
  (bind _returnvalue (Transformation|GetActorLocation))
  (Utilities|FlowControl|Sequence
    (:then_0
      (Variables|Default|SetLockedX (.X (Math|Vector|BreakVector _returnvalue))))
    (:then_1
      (Variables|Default|SetStartLocation _returnvalue))))